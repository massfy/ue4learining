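; Player character Blueprint that makes one of three weapons appear with a dissolve effect.
; WeaponAppear picks the weapon by CurrentWeaponNum, spawns it through the parent's WeaponSpawn, then plays a timeline into MP_Dissolve, reversing it after a short retriggerable delay.
; The dissolve parameter is shared; an author note reports broken appearances after the first.
; MovewithMovableActor shifts the capsule along a given direction at constant speed, with debug prints.
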(event `self.ReceiveBeginPlay`
  (`PrimitiveComponent.SetMaterial` (`self.Weapon_1`) 0 "/Game/TextOne/Materials/BP_Dissolve_Inst.BP_Dissolve_Inst")
  (`PrimitiveComponent.SetMaterial` (`self.Weapon_2`) 0 "/Game/TextOne/Materials/BP_Dissolve_Inst.BP_Dissolve_Inst")
  (`PrimitiveComponent.SetMaterial` (`self.Weapon_3`) 0 "/Game/TextOne/Materials/BP_Dissolve_Inst.BP_Dissolve_Inst"))

(event `self.WeaponAppear`
  ;[1 1 1] 现在的问题是共享存活时间导致除了第一次武器显现外均不正常
  (switch `EWeapon` (`self.CurrentWeaponNum`)
    (:`EW_Weapon1`
      (set `self.WeaponToEquip` "/Game/TextOne/Blueprint/Weapon/Weapon_test.Weapon_test_C"))
    (:`EW_Weapon2`
      (set `self.WeaponToEquip` "/Game/TextOne/Blueprint/Weapon/Weapon2.Weapon2_C"))
    (:`EW_Weapon3`
      (set `self.WeaponToEquip` "/Game/TextOne/Blueprint/Weapon/Weapon3.Weapon3_C")))
  (`self.WeaponSpawn` (`self.WeaponToEquip`))
  (set `self.WeaponOnScreen` true)
  (bind (_direction `_新建轨道_0`) (`Timeline|时间轴_0` :!via `PlayFromStart` :!label _label)
    (:`Update`
      (`KismetMaterialLibrary.SetScalarParameterValue` "/Game/TextOne/Materials/MP_Dissolve.MP_Dissolve" "Dissolve" `_新建轨道_0`)
      (`KismetSystemLibrary.RetriggerableDelay` 0.1)
      (goto _label :!via `Reverse`))))

(event `self.WeaponSpawn`
  (params (PawnClass :type "Object Class Reference"))
  (`parent.WeaponSpawn` PawnClass))

(event `self.MoveWithMovableActor`
  (params (Dir :type "Vector Structure"))
  (bind (_returnvalue_location _returnvalue_rotation _returnvalue_scale) (`KismetMathLibrary.BreakTransform` (`SceneComponent.K2_GetComponentToWorld` (`self.CapsuleComponent`))))
  (`KismetSystemLibrary.PrintString` "Hello")
  (`SceneComponent.K2_SetWorldTransform` (`self.CapsuleComponent`) (`KismetMathLibrary.MakeTransform` (+ _returnvalue_location (* (* (`GameplayStatics.GetWorldDeltaSeconds`) 250.0) (`KismetMathLibrary.Normal` Dir))) _returnvalue_rotation _returnvalue_scale) false false)
  (`KismetSystemLibrary.PrintString` "11111111111"))

(fn `UserConstructionScript`)