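; MyActor1 is an actor that moves vertically under acceleration and explodes when it reaches ground level at world Z zero, like a falling bomb.
; Each Tick adds acceleration A to Speed and offsets its Z location by that speed, scaled by delta time.
; At or below the Z threshold it destroys itself and spawns an explosion particle and sound at its location.
; A transform-reset node is left unconnected.
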(event `self.ReceiveBeginPlay`)

(event `self.ReceiveTick`
  (params (DeltaSeconds :type "Float (single-precision)"))
  (bind (_returnvalue_x _returnvalue_y _returnvalue_z) (`KismetMathLibrary.BreakVector` (`self.K2_GetActorLocation`)))
  (bind _returnvalue (`self.K2_GetActorLocation`))
  (bind (_returnvalue_x_2 _returnvalue_y_2 _returnvalue_z_2) (`KismetMathLibrary.BreakVector` (`self.K2_GetActorLocation`)))
  (bind _output_get (set `self.speed` (+ (`self.speed`) (* (`self.a`) DeltaSeconds))))
  (`self.K2_SetActorLocation` (`KismetMathLibrary.MakeVector` _returnvalue_x_2 _returnvalue_y_2 (+ _returnvalue_z_2 (* DeltaSeconds _output_get))))
  (if (<= _returnvalue_z 0.001)
    (`self.K2_DestroyActor`)
    (`GameplayStatics.SpawnEmitterAtLocation` "/Game/StarterContent/Particles/P_Explosion.P_Explosion" _returnvalue)
    (`GameplayStatics.SpawnSoundAtLocation` "/Game/StarterContent/Audio/Explosion_Cue.Explosion_Cue" _returnvalue (struct) 1.0 1.0 0.0 null null)))

(fn `UserConstructionScript`)